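; Commander camera pawn for an RTS-style build mode, possessed from a commander console, that puts the soldier in third person and shows the build menu.
; Provides planar movement with sprint, middle-mouse rotation and smoothed spring-arm zoom.
; While previewing a building, Tick traces the cursor to a grid-snapped spot, applies Q/E rotation and writes the rebased transform to the controller's pending construction info.
; Preview overlaps toggle placement validity and material.
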(event `self.ReceivePossessed`
  (params (NewController :type "Controller Object Reference"))
  ;[1 1 1] Possession
  (`self.SetOwner` NewController)
  (`self.OnClientPossess`)
  (bind _asbp_rts_player_controller (cast `/SATCOM/Core/BP_RTS_PlayerController` NewController))
  (bind _output_get (set `self.RTSPlayerControllerRef` _asbp_rts_player_controller))
  (set `/SATCOM/Core/BP_RTS_PlayerController.CommanderCamPawnRef` self _output_get))

(event `OnClientPossess`
  (bind _returnvalue (`GameplayStatics.GetPlayerController` 0))
  ;[1 1 1] Possession
  (`self.SetOwner` _returnvalue)
  (bind _asbp_rts_player_controller (cast `/SATCOM/Core/BP_RTS_PlayerController` _returnvalue))
  (bind _output_get (set `self.RTSPlayerControllerRef` _asbp_rts_player_controller))
  (set `/SATCOM/Core/BP_RTS_PlayerController.CommanderCamPawnRef` self _output_get)
  (bind _assqplayer_state (cast `SQPlayerState` (`Controller.PlayerState` _output_get)))
  (bind _assqsoldier_new (cast `SQSoldierNew` (`SQPlayerState.GetSoldier` _assqplayer_state)))
  (bind _output_get_2 (set `self.SQSoldierRef` _assqsoldier_new))
  (`MovementComponent.StopMovementImmediately` (`SQSoldier.SoldierMovement` _output_get_2))
  (if (not (`SQSoldier.bInThirdPersonView` (`self.SQSoldierRef`)))
    (`SQSoldierNew.ToggleThirdPersonView` (`self.SQSoldierRef`)))
  (`/Game/Gameplay/BP_GameplayFunctionLibrary.Show Hide Mouse` null true true true true "buildui")
  (if (not (`KismetSystemLibrary.IsValid` (`self.CommanderMainWidgetRef`)))
    (bind _commanderconsoleref (`self.CommanderConsoleRef`)
      (:`then`
        (bind _returnvalue_2 (`|CreateWidget` "/SATCOM/UserInterface/W_CommanderMain.W_CommanderMain_C" (`self.RTSPlayerControllerRef`) (`/SATCOM/Commander/BP_CommanderConsole.BuildingsAllowedForConstruction` _commanderconsoleref)))
        (set `self.CommanderMainWidgetRef` _returnvalue_2)
        (`UserWidget.AddToViewport` (`self.CommanderMainWidgetRef`) 0 :!label _label))
      (:`else`
        (`KismetSystemLibrary.PrintString` "Error: CommanderCam Pawn could not find the console" true true (struct :`R` 1.0 :`B` 0.016666 :`A` 1.0) 5.0)))
    (else
      (`Widget.SetVisibility` (`self.CommanderMainWidgetRef`) "Visible") ; If we already loaded the CommanderMain Menu,\nwe just need to un-hide it
      (if (not (`Widget.IsInViewport` (`self.CommanderMainWidgetRef`)))
        (goto _label)))))

(event `Key|E`
  (params (Key :type "Key Structure"))
  (bind (_previewbuildingrotation_roll _previewbuildingrotation_pitch _previewbuildingrotation_yaw) (`KismetMathLibrary.BreakRotator` (`self.PreviewBuildingRotation`)))
  ;[1 1 1] PreviewRotation
  (:`Pressed`
    (set `self.PreviewBuildingRotation` (`KismetMathLibrary.MakeRotator` _previewbuildingrotation_roll _previewbuildingrotation_pitch (+ _previewbuildingrotation_yaw (`self.BuildingRotationAngleSnap`))))))

(event `InputAction|Interact`
  (params (Key :type "Key Structure"))
  ;[1 1 1] Unpossession
  (:`Pressed`
    (`self.OnClientUnpossess`)))

(event `Key|Q`
  (params (Key :type "Key Structure"))
  (bind (_previewbuildingrotation_roll _previewbuildingrotation_pitch _previewbuildingrotation_yaw) (`KismetMathLibrary.BreakRotator` (`self.PreviewBuildingRotation`)))
  ;[1 1 1] PreviewRotation
  (:`Pressed`
    (set `self.PreviewBuildingRotation` (`KismetMathLibrary.MakeRotator` _previewbuildingrotation_roll _previewbuildingrotation_pitch (- _previewbuildingrotation_yaw (`self.BuildingRotationAngleSnap`))))))

(event `OnClientUnpossess`
  ;[1 1 1] Unpossession
  (if (`SQSoldier.bInThirdPersonView` (`self.SQSoldierRef`))
    (`SQSoldierNew.ToggleThirdPersonView` (`self.SQSoldierRef`)))
  (`/Game/Gameplay/BP_GameplayFunctionLibrary.Show Hide Mouse` null true false false false "buildui")
  (`self.OnServerUnpossess`))

(event `OnServerUnpossess`
  ;[1 1 1] Unpossession
  (`/SATCOM/Commander/BP_CommanderConsole.OperateCommanderConsole` (`self.CommanderConsoleRef`) false (`self.RTSPlayerControllerRef`))
  (`self.SetOwner` null))

(event `Key|MouseScrollUp`
  (params (Key :type "Key Structure"))
  ;[1 1 1] Camera Zoom
  (:`Pressed`
    (set `self.DesiredSpringArmLength` (`KismetMathLibrary.FClamp` (- (`self.DesiredSpringArmLength`) (`self.ZoomStepAmount`)) (`self.MinCameraSpringArmLength`) (`self.MaxCameraSpringArmLength`)))))

(event `Key|MouseScrollDown`
  (params (Key :type "Key Structure"))
  ;[1 1 1] Camera Zoom
  (:`Pressed`
    (set `self.DesiredSpringArmLength` (`KismetMathLibrary.FClamp` (+ (`self.DesiredSpringArmLength`) (`self.ZoomStepAmount`)) (`self.MinCameraSpringArmLength`) (`self.MaxCameraSpringArmLength`)))))

(event `self.ReceiveBeginPlay`
  ;[0.008445 1 0.03631] BeginPlay
)

(event `StartPreviewingBuilding`
  (params (PreviewMesh :type "StaticMesh Object Reference"))
  ;[1 1 1] StartPreviewingBuilding
  (`StaticMeshComponent.SetStaticMesh` (`self.BuildingPreviewStaticMeshComponent`) PreviewMesh)
  (set `self.PreviewingBuilding` true)
  (`SceneComponent.SetVisibility` (`self.BuildingPreviewStaticMeshComponent`) (`self.PreviewingBuilding`) false :!label _label_2))

(event `Key|MiddleMouseButton`
  (params (Key :type "Key Structure"))
  (bind (_returnvalue_roll _returnvalue_pitch _returnvalue_yaw) (`KismetMathLibrary.BreakRotator` (`self.K2_GetActorRotation`)))
  ;[1 1 1] Camera Rotation
  (:`Pressed`
    (goto _label_3 :!via `Open`))
  (:`Released`
    (goto _label_3 :!via `Close`)))

(event `InputAxisKey|MouseX`
  (params (AxisValue :type "Float (single-precision)"))
  (bind (_returnvalue_roll _returnvalue_pitch _returnvalue_yaw) (`KismetMathLibrary.BreakRotator` (`self.K2_GetActorRotation`)))
  ;[1 1 1] Camera Rotation
  (`/Engine/EditorBlueprintResources/StandardMacros.Gate` true :!label _label_3
    (:`Exit`
      (`self.K2_SetActorRotation` (`KismetMathLibrary.MakeRotator` _returnvalue_roll _returnvalue_pitch (+ _returnvalue_yaw (* AxisValue (`self.CameraRotationSpeed`))))))))

(event `InputAction|Sprint`
  (params (Key :type "Key Structure"))
  ;[1 1 1] Sprinting
  (:`Pressed`
    (set `FloatingPawnMovement.MaxSpeed` (* (`self.DefaultMovementSpeed`) (`self.SprintMultiplier`)) (`self.FloatingPawnMovement`)))
  (:`Released`
    (set `FloatingPawnMovement.MaxSpeed` (`self.DefaultMovementSpeed`) (`self.FloatingPawnMovement`))))

(event `StopPreviewingBuilding`
  ;[1 1 1] StartPreviewingBuilding
  (set `self.PreviewingBuilding` false)
  (goto _label_2))

(event `Key|MiddleMouseButton`
  (params (Key :type "Key Structure"))
  (bind (_returnvalue_roll _returnvalue_pitch _returnvalue_yaw) (`KismetMathLibrary.BreakRotator` (`self.K2_GetActorRotation`)))
  ;[1 1 1] Camera Rotation
  (:`Pressed`
    (goto _label_4 :!via `Open`))
  (:`Released`
    (goto _label_4 :!via `Close`)))

(event `InputAxisKey|MouseY`
  (params (AxisValue :type "Float (single-precision)"))
  (bind (_returnvalue_roll _returnvalue_pitch _returnvalue_yaw) (`KismetMathLibrary.BreakRotator` (`self.K2_GetActorRotation`)))
  ;[1 1 1] Camera Rotation
  (`/Engine/EditorBlueprintResources/StandardMacros.Gate` true :!label _label_4
    (:`Exit`
      (`self.K2_SetActorRotation` (`KismetMathLibrary.MakeRotator` _returnvalue_roll (`KismetMathLibrary.FClamp` (+ _returnvalue_pitch (* AxisValue (`self.CameraRotationSpeed`))) -10.0 40.0) _returnvalue_yaw)))))

(event `self.ReceiveTick`
  (params (DeltaSeconds :type "Float (single-precision)"))
  (bind _previewbuildingrotation (`self.PreviewBuildingRotation`))
  ;[1 0 0.01667] Tick
  (`|ExecutionSequence`
    (:`then_0`
      (`self.ManageMovement`))
    (:`then_1`
      (`self.SmoothCameraSpringArm`))
    (:`then_2`
      (if (`self.PreviewingBuilding`)
        (bind _rtsplayercontrollerref (`self.RTSPlayerControllerRef`)
          (:`then`
            (bind (_worldlocation _worlddirection) (`PlayerController.DeprojectMousePositionToWorld` _rtsplayercontrollerref))
            (bind _buildablecursowrworldposition (`self.GetCursorWorldBuildablePosition` 100000.0 "None" _worldlocation _worlddirection 500.0))
            (`SceneComponent.K2_SetWorldTransform` (`self.BuildingPreviewStaticMeshComponent`) (`KismetMathLibrary.MakeTransform` _buildablecursowrworldposition _previewbuildingrotation) true false)
            (setmembers `/SATCOM/Commander/S_BuildingConstructionInfo` :`StructRef` (`/SATCOM/Core/BP_RTS_PlayerController.PendingConstructionInfo` (`self.RTSPlayerControllerRef`)) :`WorldTransform` (`KismetMathLibrary.MakeTransform` (`GameplayStatics.RebaseLocalOriginOntoZero` _buildablecursowrworldposition) _previewbuildingrotation)))
          (:`else`
            (`KismetSystemLibrary.PrintString` "Error: CommandCam couldn't find PlayerController" true true (struct :`R` 1.0 :`B` 0.016666 :`A` 1.0) 5.0)))))))

(event `self.BuildingPreviewStaticMeshComponent.OnComponentBeginOverlap`
  (params (OverlappedComponent :type "PrimitiveComponent Object Reference") (OtherActor :type "Actor Object Reference") (OtherComp :type "PrimitiveComponent Object Reference") (OtherBodyIndex :type Integer) (bFromSweep :type Boolean) (SweepResult :type "HitResult Structure (by ref)"))
  (`PrimitiveComponent.SetMaterial` (`self.BuildingPreviewStaticMeshComponent`) 0 "/SATCOM/MaterialLibrary/MM_BadPlacement.MM_BadPlacement")
  (set `self.IsValidPlacement` false))

(event `self.BuildingPreviewStaticMeshComponent.OnComponentEndOverlap`
  (params (OverlappedComponent :type "PrimitiveComponent Object Reference") (OtherActor :type "Actor Object Reference") (OtherComp :type "PrimitiveComponent Object Reference") (OtherBodyIndex :type Integer))
  (`PrimitiveComponent.SetMaterial` (`self.BuildingPreviewStaticMeshComponent`) 0 "/SATCOM/MaterialLibrary/MM_GoodPlacement.MM_GoodPlacement")
  (set `self.IsValidPlacement` true))

(fn `GetCursorWorldBuildablePosition`
  (params (CollisionCheckDistance :type "Float (double-precision)") (DragDebugType :type "EDrawDebugTrace Enum" :default "None") (CursorWorldLocation :type "Vector Structure") (CursorWorldDirection :type "Vector Structure") (GridSnapSize :type "Float (double-precision)"))
  (returns (BuildableCursowrWorldPosition :type "Vector Structure"))
  (bind _gridsnapsize (`local.GridSnapSize`))
  (bind _outhit (`KismetSystemLibrary.LineTraceSingleForObjects` :`Start` CursorWorldLocation :`End` (+ CursorWorldLocation (* CursorWorldDirection CollisionCheckDistance)) :`ObjectTypes` (`|MakeArray` (enumliteral `EObjectTypeQuery` "ObjectTypeQuery1")) :`DrawDebugType` DragDebugType))
  (if (!= (`.HitActor` (`GameplayStatics.BreakHitResult` _outhit)) null)
    (bind _returnvalue (`KismetMathLibrary.MakeVector` (`KismetMathLibrary.GridSnap_Float` (.x (`.Location` (`GameplayStatics.BreakHitResult` _outhit))) _gridsnapsize) (`KismetMathLibrary.GridSnap_Float` (.y (`.Location` (`GameplayStatics.BreakHitResult` _outhit))) _gridsnapsize) (.z (`.Location` (`GameplayStatics.BreakHitResult` _outhit)))))
    (`KismetSystemLibrary.PrintString` (`KismetStringLibrary.Conv_VectorToString` _returnvalue) true true (struct :`R` 1.0 :`B` 0.016666 :`A` 1.0) 0.0)
    (`KismetSystemLibrary.DrawDebugSphere` _returnvalue 1000.0 12 (struct :`R` 1.0 :`B` 0.016666 :`A` 1.0))
    (return _returnvalue)))

(fn `GetTeamId`
  (returns (ReturnValue :type Integer))
  (return 0))

(fn `ManageMovement`
  (bind _rtsplayercontrollerref (`self.RTSPlayerControllerRef`)
    (:`then`
      (if (`Controller.IsLocalPlayerController` _rtsplayercontrollerref)
        (if (or (!= (`self.GetInputAxisValue`) 0.0) (!= (`self.GetInputAxisValue`) 0.0))
          (`self.AddMovementInput` (+ (* (`self.GetActorForwardVector`) (`self.GetInputAxisValue`)) (* (`self.GetActorRightVector`) (`self.GetInputAxisValue`)))))))
    (:`else`)))

(fn `SmoothCameraSpringArm`
  (set `SpringArmComponent.TargetArmLength` (`KismetMathLibrary.FInterpTo` (`SpringArmComponent.TargetArmLength` (`self.SpringArm`)) (`self.DesiredSpringArmLength`) (`GameplayStatics.GetWorldDeltaSeconds`) (`self.CameraSpringArmInterpolationSpeed`)) (`self.SpringArm`)))

(fn `UserConstructionScript`)