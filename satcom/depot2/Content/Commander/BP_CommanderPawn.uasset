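; Commander pawn that the player rotates by holding the middle mouse button, and that reports a team ID.
; It sets a fixed starting rotation on BeginPlay.
; A Gate, opened and closed by the middle mouse button, passes the scaled Turn axis into world yaw rotation.
; GetTeamId forwards to GetTeamIdMessage on player controller 0, so it always reflects that controller rather than the pawn's own.
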(event `self.ReceiveBeginPlay`
  (`self.K2_SetActorRotation` (struct :`Yaw` -90.0)))

(event `InputAxis|Turn`
  (params (AxisValue :type "Float (single-precision)"))
  (`/Engine/EditorBlueprintResources/StandardMacros.Gate` true :!label _label
    (:`Exit`
      (`self.K2_AddActorWorldRotation` (`KismetMathLibrary.MakeRotator` 0.0 0.0 (* AxisValue 5.0))))))

(event `Key|MiddleMouseButton`
  (params (Key :type "Key Structure"))
  (:`Pressed`
    (goto _label :!via `Open`))
  (:`Released`
    (goto _label :!via `Close`)))

(fn `GetTeamId`
  (returns (ReturnValue :type Integer))
  (bind _returnvalue (message `SQTeamInterface.GetTeamId` (`GameplayStatics.GetPlayerController` 0)))
  (return _returnvalue))

(fn `UserConstructionScript`
  (`parent.UserConstructionScript`))