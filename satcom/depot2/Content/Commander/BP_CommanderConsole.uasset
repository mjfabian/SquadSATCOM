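; BP_CommanderConsole is a usable console that lets a player take control of a commander camera pawn.
; On BeginPlay the server spawns a BP_CommanderCam and gives it a back-reference to the console, which an OnRep function also sets.
; Using the console possesses the camera and halts the user's soldier.
; OperateCommanderConsole also handles exit, repossessing the soldier if alive or unpossessing if dead.
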(event `self.ReceiveBeginPlay`
  ;[0.008445 1 0.03631] Create a CommanderCam Pawn
  (`/Engine/EditorBlueprintResources/ActorMacros.Switch Has Authority`
    (:`Authority`
      (bind _returnvalue (`|SpawnActorFromClass` "/SATCOM/Commander/BP_CommanderCam.BP_CommanderCam_C" (`self.EmptyTransform`) "AlwaysSpawn" "OverrideRootScale" null null))
      (`KismetSystemLibrary.PrintString` (`KismetStringLibrary.Concat_StrStr` (`KismetSystemLibrary.GetDisplayName` self) " spawned a CommanderCam") true true (struct :`R` 0.008445 :`G` 1.0 :`B` 0.036314 :`A` 1.0) 10.0)
      (set `self.CommanderCam` _returnvalue)
      (set `/SATCOM/Commander/BP_CommanderCam.CommanderConsoleRef` self (`self.CommanderCam`)) ; Pass a reference to this console\non to the new CommanderCam
    )))

(event `self.ServerOnUsed`
  (params (User :type "Controller Object Reference"))
  (bind _asplayer_controller (cast `PlayerController` User))
  (`self.OperateCommanderConsole` true _asplayer_controller))

(fn `OnRep_CommanderCamTest`
  (set `/SATCOM/Commander/BP_CommanderCam.CommanderConsoleRef` self (`self.CommanderCam`)))

(fn `OperateCommanderConsole`
  (params (Operate :type Boolean) (PlayerController :type "PlayerController Object Reference"))
  (locals (PlayerStateSoldierLocal :type "SQSoldier Object Reference"))
  ;[1 1 1] Get the Soldier
  (bind _assqplayer_state (cast `SQPlayerState` (`Controller.PlayerState` PlayerController))
    (:`then`
      (bind _returnvalue (`SQPlayerState.GetSoldier` _assqplayer_state))
      (`/Engine/EditorBlueprintResources/StandardMacros.IsValid` _returnvalue
        (:`Is Valid`
          (set `local.PlayerStateSoldierLocal` _returnvalue) ; Save player's PlayerState's, Soldier to a local variable
          (if (`local.Operate`)
            ;[1 1 1] Operating the console
            (`Controller.Possess` (`local.PlayerController`) (`self.CommanderCam`)) ; When we USE this actor, take the incoming playercontroller\nand tell it to possess the CommanderPawn,
            (`MovementComponent.StopMovementImmediately` (`SQSoldier.SoldierMovement` (`local.PlayerStateSoldierLocal`))) ; and stop the soldier's movement
            (else
              ;[1 1 1] Stop Operating
              (if (`SQSoldier.IsAlive` (`local.PlayerStateSoldierLocal`))
                (`Controller.Possess` (`local.PlayerController`) (`local.PlayerStateSoldierLocal`)) ; When we stop operating the console,\nIf the user is still alive, posses the soldier again
                (else
                  (`Controller.UnPossess` (`local.PlayerController`)) ; If we're dead, just unpossess the CommanderConsole
                )))))))
    (:`CastFailed`
      (`KismetSystemLibrary.PrintString` "Error: CommanderConsolder failed to find user's SQPlayerState" true true (struct :`R` 1.0 :`B` 0.016666 :`A` 1.0) 5.0))))

(fn `UserConstructionScript`
  (`parent.UserConstructionScript`))