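; BP_BuildingMaster is a base building actor with health, a team ID and an optional construction phase.
; BeginPlay seeds the HealthComponent from initial and max health and applies the configured static mesh.
; A positive ConstructionTime hides the mesh, disables its collision and shows the ConstructionZone; otherwise the finished, collidable building appears.
; Construction progress and cost are not handled in this graph, and GetTeamId exposes the team.
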(event `self.ReceiveBeginPlay`
  (bind _healthcomponent (`self.HealthComponent`))
  (set `/Game/Blueprints/AI/AutomatedWeapons/HealthComponent.Health` (`self.InitialHealth`) (`self.HealthComponent`))
  (set `/Game/Blueprints/AI/AutomatedWeapons/HealthComponent.Max Health` (`self.MaxHealth`) _healthcomponent)
  (`ActorComponent.Activate` _healthcomponent false)
  (`StaticMeshComponent.SetStaticMesh` (`self.BuildingStaticMeshComponent`) (`self.BuildingStaticMesh`))
  (if (> (`self.ConstructionTime`) 0.0)
    (`SceneComponent.SetVisibility` (`self.BuildingStaticMeshComponent`) false false)
    (`PrimitiveComponent.SetCollisionEnabled` (`self.BuildingStaticMeshComponent`) "NoCollision")
    (`SceneComponent.SetVisibility` (`self.ConstructionZone`) true true)
    (else
      (`SceneComponent.SetVisibility` (`self.BuildingStaticMeshComponent`) true false)
      (`PrimitiveComponent.SetCollisionEnabled` (`self.BuildingStaticMeshComponent`) "QueryAndPhysics")
      (`SceneComponent.SetVisibility` (`self.ConstructionZone`) false true))))

(fn `GetTeamId`
  (returns (ReturnValue :type Integer))
  (return (`self.TeamID`)))

(fn `UserConstructionScript`)