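; RTS player controller for a Squad-based mode where a team's commander spawns in a bunker and places buildings.
; On team change it binds to the team's CommanderState and finds a friendly bunker spawn.
; A commander change respawns both players involved, sending the new one to the bunker and emptying and locking their squad.
; Left click spawns the pending building with origin rebasing for the client-sent location; right click cancels the preview.
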(event `FindCommanderSpawn`
  ;[1 1 1] Find a friendly CommanderSpawnBunker
  (`|ExecutionSequence`
    (:`then_0`
      (bind _outactors (`GameplayStatics.GetAllActorsOfClass` "/SATCOM/Commander/BP_CommanderBunkerSpawn.BP_CommanderBunkerSpawn_C"))
      (for _array_element _outactors
        (if (== (`SQTeamInterface.GetTeamId` _array_element) (`self.GetTeam`))
          (set `self.CommanderBunkerSpawn` _array_element)
          (break)))
      (`self.CommanderBunkerSpawn`
        (:`then`)
        (:`else`
          (`KismetSystemLibrary.PrintString` "Error: Could not find a (friendly) CommanderBunkerSpawn in the level" true true (struct :`R` 1.0 :`B` 0.016666 :`A` 1.0) 10.0))))
    (:`then_1`)))

(event `SQTeamInterface.OnTeamChange`
  (params (PreviousTeam :type Integer))
  (bind _returnvalue (`self.GetTeam`))
  (bind _indexedteamstates (`SQGameState.IndexedTeamStates` (`/Game/Gameplay/BP_GameplayFunctionLibrary.GetSquadGameState`)))
  ;[1 1 1] Bind custom event to CommanderState's
  ; "CommanderChanged" event dispatcher
  (if (`KismetArrayLibrary.Array_IsValidIndex` _indexedteamstates _returnvalue)
    (add `SQCommanderState.OnCommanderChangedEvent` (`SQTeamState.CommanderState` (`|GetArrayItem` _indexedteamstates _returnvalue)) (`|CreateDelegate` :!event `CommanderChanged`)) ; Whenever that CommanderState fires an event dispatcher\nsaying that the commander changed, we will fire our own \n"CommanderChanged" custom event
    (`self.FindCommanderSpawn`)))

(event `Key|RightMouseButton`
  (params (Key :type "Key Structure"))
  ;[1 1 1] Right Click
  (:`Pressed`
    (bind _commandercampawnref (`self.CommanderCamPawnRef`)
      (:`then`
        (`/SATCOM/Commander/BP_CommanderCam.StopPreviewingBuilding` _commandercampawnref)
        (set `self.IsPlacingBuilding` false))
      (:`else`))))

(event `CommanderChanged`
  (params (`Old Commander SQPlayerState` :type "SQPlayerState Object Reference") (`New Commander SQPlayerState` :type "SQPlayerState Object Reference"))
  ;[1 1 1] Respawn commander in bunker
  (if (== `New Commander SQPlayerState` (`self.PlayerState`))
    (`self.Respawn`)
    (`self.ServerRequestRestartPlayer` (`self.CommanderBunkerSpawn`)) ; Spawn the player in the Commander Bunker
    (`self.ClearCommanderSquad`) ; and empty our their squad
    (elif (== `Old Commander SQPlayerState` (`self.PlayerState`))
      (`self.Respawn`) ; Let the former commander respawn and join the fight
    )))

(event `Key|LeftMouseButton`
  (params (Key :type "Key Structure"))
  ;[1 1 1] Left Click
  (:`Pressed`
    (if (and (`self.IsCommander`) (`self.IsPlacingBuilding`))
      (`self.SpawnBuilding` (`self.PendingConstructionInfo`)))))

(event `ClearCommanderSquad`
  ;[1 1 1] Remove all players from squad and lock it
  (if (`self.IsSquadLeader`)
    (bind _squadstate (`self.SquadState`)
      (:`then`
        (for _array_element (`SQSquadState.PlayerStates` _squadstate)
          (if (!= _array_element (`self.PlayerState`))
            (`self.KickPlayerFromSquad` _array_element) ; For each playerstate that is NOT this one,\nkick it from our squad
          ))
        (if (not (`SQSquadState.bIsLocked` _squadstate))
          (`self.ServerChangeSquadLock` null) ; Once completed, if the squad isn't locked, lock it.
        ))
      (:`else`))))

(event `SpawnBuilding`
  (params (ConstructionInfo :type "/SATCOM/Commander/S_BuildingConstructionInfo Structure"))
  (bind _returnvalue (`KismetMathLibrary.MakeTransform` (`GameplayStatics.RebaseZeroOriginOntoLocal` (.location ConstructionInfo_WorldTransform_42_68D2E5B540C80FCE6F31EAA0CFCA0B11)) (.rotation ConstructionInfo_WorldTransform_42_68D2E5B540C80FCE6F31EAA0CFCA0B11) (.scale ConstructionInfo_WorldTransform_42_68D2E5B540C80FCE6F31EAA0CFCA0B11)))
  ;[1 1 1] Spawn a Building
  (if (`KismetSystemLibrary.IsValidClass` ConstructionInfo_Class_31_4968A07A42E19FA7F446F58F970EFCC2)
    (bind _returnvalue_2 (`|SpawnActorFromClass` ConstructionInfo_Class_31_4968A07A42E19FA7F446F58F970EFCC2 _returnvalue "AlwaysSpawn" "OverrideRootScale" (`self.GetOwner`) (`self.GetTeam`) ConstructionInfo_ConstructionTime_9_18852AA543A99FC28D320C989547F823 ConstructionInfo_MaxHealth_47_0934138E4357E14BD7CD89A6823C9311 ConstructionInfo_MaxHealth_47_0934138E4357E14BD7CD89A6823C9311 ConstructionInfo_BuildingMesh_49_AB0BB8584342E51FB73102A45D23BB4E null)) ; Use our location sent from the client who triggered this event,\nrebase it to our server's local origin, and use the rotation that they sent\n(by Q / E rotating the preview). Take this transform and skeletal mesh \nand use it to spawn a new building
    (set `self.IsPlacingBuilding` false)
    ;;[0 0.3688 1] Debug
    (`KismetSystemLibrary.PrintString` (`KismetStringLibrary.Concat_StrStr` "Spawned a " (`KismetSystemLibrary.GetDisplayName` _returnvalue_2) " at " (`KismetStringLibrary.Conv_VectorToString` (.location _returnvalue))) true true (struct :`R` 0.008445 :`G` 1.0 :`B` 0.036314 :`A` 1.0) 10.0)))

(fn `UserConstructionScript`
  (`parent.UserConstructionScript`))